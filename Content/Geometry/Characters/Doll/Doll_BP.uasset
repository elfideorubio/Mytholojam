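; Doll character Blueprint that wanders the nav mesh and reacts when it sees the player.
; From BeginPlay it repeatedly moves to random navigable points nearby, pausing briefly after each successful move.
; When PawnSensing sees a pawn, it starts moving toward player 0.
; On the first sighting only, it also plays a voice sound, then after a short delay ragdolls its mesh from the pelvis down.
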(event OnSeePawn(PawnSensing)
  (params (Pawn :type Pawn%20Object%20Reference))
  (bind _returnvalue (Game|GetPlayerCharacter 0))
  (AI|AIMoveTo self (Transformation|GetActorLocation _returnvalue) _returnvalue 5.0 false
    (:then
      (Utilities|FlowControl|DoOnce false
        (:Completed
          (Audio|PlaySound2D "/Game/Sound/03_VO/Kikimora_drafts/dollvoice.dollvoice" 1.0 1.0 0.0 0 0)
          (Utilities|FlowControl|Delay 1.0)
          (Class|SkeletalMeshComponent|SetAllBodiesBelowSimulatePhysics (Variables|Character|GetMesh) (Utilities|Name|MakeLiteralName "Pelvis") true true))))))

(event Custom|MoveToRandomLocation
  ;[1 1 1] moving to a random spot on nav mesh
  (AI|AIMoveTo self (.RandomLocation (Class|NavigationSystemV1|GetRandomPointinNavigableRadius (Transformation|GetActorLocation) 5e+02 0 0)) 0 5.0 false
    (:OnSuccess
      (Utilities|FlowControl|Delay 0.8)
      (CallFunction|MovetoRandomLocation))))

(event EventBeginPlay
  (CallFunction|MovetoRandomLocation))

(event Collision|EventActorBeginOverlap
  (params (OtherActor :type Actor%20Object%20Reference)))

(event EventTick
  (params (DeltaSeconds :type Float%20%28single-precision%29)))

(fn ConstructionScript)