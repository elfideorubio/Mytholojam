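; Doll Blueprint that checks whether every Trace actor in the level is named "Prison", with no action yet attached to the result.
; BeginPlay caches all Trace actors and binds Update to a looping timer with zero time, which Unreal does not schedule.
; Update sets the Spawned flag only if all cached actors match, then stops re-checking, but its success branch is empty.
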(event Custom|Update
  (if (not (Variables|Default|GetSpawned))
    (Variables|Default|SetSpawned true)
    (for _array_element (Variables|Default|GetTrace)
      (if (not (Utilities|Enum|Equal(Enum) (Variables|/Game/Blueprint/Assets/Glyph/Glyph.Glyph_C|GetName _array_element) "Prison"))
        (Variables|Default|SetSpawned false)))
    (if (Variables|Default|GetSpawned)
      _)))

(event EventBeginPlay
  (bind _outactors (Actor|GetAllActorsOfClass "/Game/Blueprint/Assets/Trace/Trace.Trace_C"))
  (Variables|Default|SetTrace _outactors)
  (Utilities|Time|SetTimerbyEvent (delegate Custom|Update) 0.0 true))

(fn ConstructionScript)