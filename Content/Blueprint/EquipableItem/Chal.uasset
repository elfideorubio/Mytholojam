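; Chal is an equipable item Blueprint whose toggle event animates its skeletal mesh between on and off states.
; Toggling on plays the mesh's animation forward from partway in, while toggling off plays it in reverse from a later position, so one animation serves both directions.
; The item action and BeginPlay events are empty, and the construction script only calls the parent.
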(event EventEquipedItemToggleActive
  (params (On/Off :type Boolean))
  (bind _skeletalmesh (Variables|Default|GetSkeletalMesh))
  (bind _skeletalmesh_2 (Variables|Default|GetSkeletalMesh))
  (if On/Off
    (Audio|Components|Audio|Play _skeletalmesh false)
    (Components|Animation|SetPosition _skeletalmesh 0.4 false)
    (Components|Timeline|SetPlayRate _skeletalmesh 1.0)
    (else
      (Audio|Components|Audio|Play _skeletalmesh_2 false)
      (Components|Animation|SetPosition _skeletalmesh_2 1.0 false)
      (Components|Timeline|SetPlayRate _skeletalmesh_2 -1.0))))

(event EventEquipedItemAction)

(event EventBeginPlay)

(fn ConstructionScript
  (|CallParentFunction))