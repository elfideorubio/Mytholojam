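; Equipable torch item that switches its point light and spot light on and off through an equipped-item toggle event.
; The event acts only when the requested state differs from LightOn, then plays the skeletal mesh animation forward or in reverse from set start positions.
; The Light_Turn_On timeline plays or reverses alongside it, scaling both light intensities, with the spot light ten times stronger.
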(event EventEquipedItemToggleActive
  (params (On/Off :type Boolean))
  (bind _skeletalmesh (Variables|Default|GetSkeletalMesh))
  (bind _skeletalmesh_2 (Variables|Default|GetSkeletalMesh))
  (if (Class|KismetMathLibrary|XORBoolean On/Off (Variables|Default|GetLightOn))
    (Variables|Default|SetLightOn (not (Variables|Default|GetLightOn)))
    (if (Variables|Default|GetLightOn)
      (Audio|Components|Audio|Play _skeletalmesh false)
      (Components|Animation|SetPosition _skeletalmesh 0.4 false)
      (Components|Timeline|SetPlayRate _skeletalmesh 1.0)
      (bind _newtrack_0 (Timeline|Light_Turn_On PlayFromStart)
        (:Update
          (Rendering|Components|Light|SetIntensity (Variables|Default|GetPointLight) (* _newtrack_0 1e+02))
          (Rendering|Components|Light|SetIntensity (Variables|Default|GetSpotLight) (* _newtrack_0 1e+03))))
      (else
        (Audio|Components|Audio|Play _skeletalmesh_2 false)
        (Components|Animation|SetPosition _skeletalmesh_2 1.0 false)
        (Components|Timeline|SetPlayRate _skeletalmesh_2 -1.0)
        (Timeline|Light_Turn_On ReverseFromEnd)))))

(fn ConstructionScript
  (|CallParentFunction))