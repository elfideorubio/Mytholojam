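; Equipable candle item that shows or hides two static meshes and a particle system when equipped or unequipped.
; BeginPlay flips their visibility once, and EquipedItemToggleActive flips it again only when the requested state differs from LightOn, printing a torch equip message.
; Visibility is toggled rather than set, so it depends on the components' default state.
; The item action event is empty.
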(event EventEquipedItemToggleActive
  (params (On/Off :type Boolean))
  (if (Class|KismetMathLibrary|XORBoolean On/Off (Variables|Default|GetLightOn))
    (Rendering|ToggleVisibility (Variables|Default|GetStaticMesh) false)
    (Rendering|ToggleVisibility (Variables|Default|GetStaticMesh1) false)
    (Rendering|ToggleVisibility (Variables|Default|GetParticleSystem) false)
    (Variables|Default|SetLightOn (not (Variables|Default|GetLightOn)))
    (if (Variables|Default|GetLightOn)
      (Development|PrintString "Equiped Torch")
      (else
        (Development|PrintString "Unequiped Torch")))))

(event EventEquipedItemAction)

(event EventBeginPlay
  (Rendering|ToggleVisibility (Variables|Default|GetStaticMesh) false)
  (Rendering|ToggleVisibility (Variables|Default|GetStaticMesh1) false)
  (Rendering|ToggleVisibility (Variables|Default|GetParticleSystem) false))

(fn ConstructionScript
  (|CallParentFunction))