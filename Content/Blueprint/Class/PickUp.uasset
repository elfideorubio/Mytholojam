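; Base pickup actor that the player collects through an interact event.
; On interact, it adds itself to the first-person character's PickUp array, then hides, disables collision and tick, flags itself as picked up and plays a pickup sound.
; The actor stays in the world rather than being destroyed, and it supplies an in-range prompt built from "Pickup" and its name.
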(event EventOnInteract
  (params (Key :type Key%20Structure))
  (bind _asfirst_person_character (Utilities|Casting|CastToFirstPersonCharacter (Game|GetPlayerCharacter 0)))
  (Utilities|Array|Add (Variables|/Game/FirstPersonBP/Blueprints/FirstPersonCharacter.FirstPersonCharacter_C|GetPickUp _asfirst_person_character) self)
  (Rendering|SetActorHiddenInGame true)
  (Collision|SetActorEnableCollision false)
  (Actor|Tick|SetActorTickEnabled false)
  (Variables|Default|SetPicked_Up true)
  (Audio|SpawnSoundatLocation "/Game/Sound/00_SoundCue_and_mixers/Item_pick_up.Item_pick_up" "0, 0, 0" "0, 0, 0" 1.0 1.0 0.0 0 0))

(fn ConstructionScript
  (|CallParentFunction))

(fn UIinRangeInteract
  (return (Utilities|Text|ToText(String) (Utilities|String|Append "Pickup " (Utilities|String|ToString(Text) (Variables|Default|GetPickup_Name))))))