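; DefaultRoom is a room actor that tracks player presence and sets its room type from its salt and glyph.
; At BeginPlay it gathers child Salt and TriggerBox actors, giving each box a nav modifier.
; A one-second looping timer updates the player's ActRoom from box overlaps, then checks salt and glyph.
; Vigilance glyph with placed salt means Safe, switching nav areas to NavKikimora while the player is inside; Power Glyph Doll means Exorcism.
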(event EventBeginPlay
  (Utilities|Time|SetTimerbyFunctionName 0 "UpdateSelfState" 1.0 true)
  (for _array_element (Actor|GetAllChildActors true)
    (bind _assalt (Utilities|Casting|CastToSalt _array_element)
      (:then
        (Utilities|Array|Add (Variables|Default|GetAllSalt) _assalt))
      (:CastFailed
        (bind _astrigger_box (Utilities|Casting|CastToTriggerBox _array_element))
        (Utilities|Array|Add (Variables|Default|GetAllRoomSpace) _astrigger_box))))
  (for _array_element_2 (Variables|Default|GetAllRoomSpace)
    (bind _returnvalue (AddComponent|AddNavModifierComponent _array_element_2))
    (Utilities|Array|Add (Variables|Default|GetAllNavModifier) _returnvalue)
    (Class|NavModifierComponent|SetAreaClass _returnvalue "/Script/NavigationSystem.NavArea_Default")))

(fn ConstructionScript)

(fn UpdateSelfState
  (bind _asfirst_person_character (Utilities|Casting|CastToFirstPersonCharacter (Game|GetPlayerCharacter 0)))
  (if (== (Variables|/Game/FirstPersonBP/Blueprints/FirstPersonCharacter.FirstPersonCharacter_C|GetActRoom _asfirst_person_character) self)
    (Variables|/Game/FirstPersonBP/Blueprints/FirstPersonCharacter.FirstPersonCharacter_C|SetActRoom _asfirst_person_character 0))
  (Variables|Default|SetPlayerIn false)
  (bind _array_element (Utilities|Array|ForEachLoopwithBreak (Variables|Default|GetAllRoomSpace) :!label _label)
    (:LoopBody
      (if (Collision|IsOverlappingActor (Variables|/Script/Engine.TriggerBase|GetCollisionComponent _array_element) (Game|GetPlayerCharacter 0) :!class /Script/Engine.PrimitiveComponent)
        (Variables|Default|SetPlayerIn true)
        (bind _asfirst_person_character_2 (Utilities|Casting|CastToFirstPersonCharacter (Game|GetPlayerCharacter 0)))
        (Variables|/Game/FirstPersonBP/Blueprints/FirstPersonCharacter.FirstPersonCharacter_C|SetActRoom _asfirst_person_character_2 self)
        (goto _label Break)))
    (:Completed
      (for _array_element_2 (Variables|Default|GetAllSalt)
        (if (not (Variables|/Game/Blueprint/Assets/Salt/Salt.Salt_C|GetPlaced _array_element_2))
          (LocalVariables|SetAllSaltPlaced false)))
      (bind _asglyph (Utilities|Casting|CastToGlyph (Variables|/Script/Engine.ChildActorComponent|GetChildActor (Variables|Default|GetGlyph))))
      (switch string (Variables|/Game/Blueprint/Assets/Glyph/Glyph.Glyph_C|GetName _asglyph)
        (:Vigilance%20Glyph
          (if (LocalVariables|GetAllSaltPlaced)
            (Variables|Default|SetRoom%20Type "Safe")
            (if (Variables|Default|GetPlayerIn)
              (for _array_element_3 (Variables|Default|GetAllNavModifier)
                (Class|NavModifierComponent|SetAreaClass _array_element_3 "/Game/Blueprint/Class/NavKikimora.NavKikimora_C")))))
        (:Power%20Glyph%20Doll
          (Variables|Default|SetRoom%20Type "Exorcism"))))))