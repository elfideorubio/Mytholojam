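; RandomSpawner is an actor Blueprint that randomly thins out placed actors of a configured Class at BeginPlay, leaving at most Number in the level.
; It gathers all actors of that Class, then repeatedly picks one at random and removes it from the list until the count no longer exceeds Number.
; Despite its name it spawns nothing, and culls each picked actor by setting a near-zero life span.
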(event EventBeginPlay
  (bind _outactors (Actor|GetAllActorsOfClass (Variables|Default|GetClass)))
  (Variables|Default|SetAllActor _outactors)
  (while (> (Utilities|Array|Length (Variables|Default|GetAllActor)) (Variables|Default|GetNumber))
    (bind _output_get (Variables|Default|SetChoosenActor (Utilities|Array|Get(acopy) (Variables|Default|GetAllActor) (Math|Random|RandomInteger (Utilities|Array|Length (Variables|Default|GetAllActor))))))
    (Utilities|Array|RemoveItem (Variables|Default|GetAllActor) _output_get)
    (Actor|SetLifeSpan (Variables|Default|GetChoosenActor) 0.01)))

(fn ConstructionScript)