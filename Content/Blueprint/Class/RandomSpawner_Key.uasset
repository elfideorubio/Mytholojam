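; RandomSpawner_Key randomizes key placement by keeping one randomly chosen Key actor per pickup type among those already in the level.
; On BeginPlay it gathers all Key actors and builds a list of their distinct PickupType values.
; It then repeatedly picks a random key and removes others of the same type through a near-zero lifespan, until the remaining key count matches the type count.
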(event EventBeginPlay
  (bind _outactors (Actor|GetAllActorsOfClass "/Game/Blueprint/Assets/PickUp/Key/Key.Key_C"))
  (bind _output_get (Variables|Default|SetAllActor _outactors))
  (for _array_element _output_get
    (bind _askey (Utilities|Casting|CastToKey _array_element))
    (if (not (Utilities|Array|ContainsItem (Variables|Default|GetType) (Variables|/Game/Blueprint/Class/PickUp.PickUp_C|GetPickup_Type _askey)))
      (Utilities|Array|Add (Variables|Default|GetType) (Variables|/Game/Blueprint/Class/PickUp.PickUp_C|GetPickup_Type _askey))))
  (while (!= (Utilities|Array|Length (Variables|Default|GetType)) (Utilities|Array|Length (Variables|Default|GetAllActor)))
    (Variables|Default|SetChoosenActor (Utilities|Array|Get(acopy) (Variables|Default|GetAllActor) (Math|Random|RandomInteger (Utilities|Array|Length (Variables|Default|GetAllActor)))))
    (for _array_element_2 (Variables|Default|GetAllActor)
      (bind _output_get_2 (Variables|Default|SetActToErase _array_element_2))
      (bind _askey_2 (Utilities|Casting|CastToKey _output_get_2))
      (bind _askey_3 (Utilities|Casting|CastToKey (Variables|Default|GetChoosenActor)))
      (if (and (!= (Variables|Default|GetChoosenActor) (Variables|Default|GetActToErase)) (Utilities|Enum|Equal(Enum) (Variables|/Game/Blueprint/Class/PickUp.PickUp_C|GetPickup_Type _askey_3) (Variables|/Game/Blueprint/Class/PickUp.PickUp_C|GetPickup_Type _askey_2)))
        (Utilities|Array|RemoveItem (Variables|Default|GetAllActor) (Variables|Default|GetActToErase))
        (Actor|SetLifeSpan (Variables|Default|GetActToErase) 0.01)))))

(fn ConstructionScript)